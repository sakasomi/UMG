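; BP_Button is an interactive switch that shows or hides the Sphere component of every actor in ObjectsArray.
; Any overlap with its Box toggles between SwitchOn and SwitchOff based on IsOn.
; Overlapping its own Sphere opens a WBP_ButtonOnOff widget holding a reference to the button and enables the mouse cursor.
; Ending that overlap removes all widgets, hides the cursor and restores game-only input.
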(event `self.Box.OnComponentBeginOverlap`
  (params (OverlappedComponent :type "PrimitiveComponent Object Reference") (OtherActor :type "Actor Object Reference") (OtherComp :type "PrimitiveComponent Object Reference") (OtherBodyIndex :type Integer) (bFromSweep :type Boolean) (SweepResult :type "HitResult Structure (by ref)"))
  (if (`self.IsOn`)
    (`self.SwitchOff`)
    (else
      (`self.SwitchOn`))))

(event `/Game/Project/Blueprints/BPI_Switchable.SwitchOff`
  (for _array_element (`self.ObjectsArray`)
    (`SceneComponent.SetVisibility` (`/Game/Project/Blueprints/BP_Object.Sphere` _array_element) false false)
    (set `self.IsOn` false)))

(event `/Game/Project/Blueprints/BPI_Switchable.SwitchOn`
  (for _array_element (`self.ObjectsArray`)
    (`SceneComponent.SetVisibility` (`/Game/Project/Blueprints/BP_Object.Sphere` _array_element) true false)
    (set `self.IsOn` true)))

(event `self.Sphere.OnComponentBeginOverlap`
  (params (OverlappedComponent :type "PrimitiveComponent Object Reference") (OtherActor :type "Actor Object Reference") (OtherComp :type "PrimitiveComponent Object Reference") (OtherBodyIndex :type Integer) (bFromSweep :type Boolean) (SweepResult :type "HitResult Structure (by ref)"))
  (bind _returnvalue (`GameplayStatics.GetPlayerController` 0))
  (cast `/Game/ThirdPerson/Blueprints/BP_ThirdPersonCharacter` (`GameplayStatics.GetPlayerCharacter` 0))
  (`WidgetBlueprintLibrary.SetInputMode_GameAndUIEx` _returnvalue null)
  (set `PlayerController.bShowMouseCursor` true _returnvalue)
  (bind _returnvalue_2 (`|CreateWidget` "/Game/Project/Blueprints/WBP_ButtonOnOff.WBP_ButtonOnOff_C"))
  (set `/Game/Project/Blueprints/WBP_ButtonOnOff.ButtonActor` self _returnvalue_2)
  (`UserWidget.AddToViewport` _returnvalue_2 0))

(event `self.Sphere.OnComponentEndOverlap`
  (params (OverlappedComponent :type "PrimitiveComponent Object Reference") (OtherActor :type "Actor Object Reference") (OtherComp :type "PrimitiveComponent Object Reference") (OtherBodyIndex :type Integer))
  (bind _returnvalue (`GameplayStatics.GetPlayerController` 0))
  (cast `/Game/ThirdPerson/Blueprints/BP_ThirdPersonCharacter` (`GameplayStatics.GetPlayerCharacter` 0))
  (`WidgetBlueprintLibrary.SetInputMode_GameOnly` _returnvalue)
  (`WidgetLayoutLibrary.RemoveAllWidgets`)
  (set `PlayerController.bShowMouseCursor` false _returnvalue))

(fn `IsVisible`
  (returns (IsOn :type Boolean))
  (return false))

(fn `UserConstructionScript`)